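; Moving platform hazard that travels along a timeline and reloads Sam_Level when anything overlaps its box.
; On BeginPlay the timeline starts at a configurable play rate and lerps the platform mesh's relative location between its origin and EndLocation.
; After each run it waits briefly and replays from the start.
; The box overlap has no actor check, although its comment intends only the player to trigger the restart.
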(event OnComponentBeginOverlap(Box)
  (params (OverlappedComponent :type Primitive%20Component%20Object%20Reference) (OtherActor :type Actor%20Object%20Reference) (OtherComp :type Primitive%20Component%20Object%20Reference) (OtherBodyIndex :type Integer) (bFromSweep :type Boolean) (SweepResult :type Hit%20Result%20Structure%20%28by%20ref%29))
  ;[1 1 1] Restarts the level if the player hits the platform.
  (Game|OpenLevel(byName) "Sam_Level"))

(event EventBeginPlay
  ;[1 1 1] Moves the platform
  (Components|Timeline|SetPlayRate (Variables|Default|GetPlatformUpDown) (Variables|Default|GetPlayRate))
  (bind _updown (Timeline|PlatformUpDown Play)
    (:Update
      (Transformation|SetRelativeLocation (Variables|Default|GetPlatform) (Math|Vector|Lerp(Vector) "0, 0, 0" (Variables|Default|GetEndLocation) _updown) false false))
    (:Finished
      (Utilities|FlowControl|Delay 0.2)
      (Timeline|PlatformUpDown PlayFromStart))))

(fn ConstructionScript)